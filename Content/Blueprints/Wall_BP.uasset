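; Modular wall actor that assembles front and back wall pieces plus front and back ceiling pieces from configurable meshes.
; The construction script adds a static mesh component for each, setting the back wall behind the front and both ceiling pieces at a shared raised, centered offset.
; Two mirror flags flip the back wall and back ceiling with negative X scale.
; The event graph has no active logic.
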(event EventBeginPlay)

(event Collision|EventActorBeginOverlap
  (params (OtherActor :type Actor%20Object%20Reference)))

(event EventTick
  (params (DeltaSeconds :type Float%20%28single-precision%29)))

(fn ConstructionScript
  (bind _returnvalue (AddComponent|AddStaticMeshComponent false))
  (Components|StaticMesh|SetStaticMesh _returnvalue (Variables|Default|GetAddFrontWall))
  (bind _returnvalue_2 (AddComponent|AddStaticMeshComponent false))
  (Components|StaticMesh|SetStaticMesh _returnvalue_2 (Variables|Default|GetAddBackWall))
  (Transformation|SetRelativeTransform _returnvalue_2 (Math|Transform|MakeTransform "-10.000000,0.000000,0.000000" "0, 0, 0" (.scale (Math|Transform|MakeTransform "0, 0, 0" "0, 0, 0" (Utilities|Select :Index (Variables|Default|GetMirrorWallMesh) :NewEnumerator0 "-1.000000,1.000000,1.000000" :NewEnumerator1 "1.000000,1.000000,1.000000")))) false false)
  (bind _returnvalue_3 (AddComponent|AddStaticMeshComponent false))
  (Components|StaticMesh|SetStaticMesh _returnvalue_3 (Variables|Default|GetAddFrontCeiling))
  (Transformation|SetRelativeTransform _returnvalue_3 (Math|Transform|MakeTransform "-5.000000, 0,35.000000" "0, 0, 0" "1,1,1") false false)
  (bind _returnvalue_4 (AddComponent|AddStaticMeshComponent false))
  (Components|StaticMesh|SetStaticMesh _returnvalue_4 (Variables|Default|GetAddBackCeiling))
  (Transformation|SetRelativeTransform _returnvalue_4 (Math|Transform|MakeTransform "-5.000000, 0,35.000000" "0, 0, 0" (.scale (Math|Transform|MakeTransform "0, 0, 0" "0, 0, 0" (Utilities|Select :Index (Variables|Default|GetMirrorCeilingMesh) :NewEnumerator0 "-1.000000,1.000000,1.000000" :NewEnumerator1 "1.000000,1.000000,1.000000")))) false false))