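; PuddleTeleporter is a puddle actor that reveals its water while the linked Sink leaks and can pull the player through to another location.
; Tick unhides the puddle, and overlap events track whether the first-person character is standing in it.
; SinkActivated disables movement, fades to black and drags the player vertically with a timeline.
; When the timeline ends, it teleports the player to fixed coordinates, fades back in and switches movement to swimming.
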(event Custom|SinkActivated
  (params (PlayerActor :type Actor%20Object%20Reference))
  (bind _asfirst_person_character (Utilities|Casting|CastToFirstPersonCharacter PlayerActor))
  (Pawn|Components|CharacterMovement|DisableMovement (Variables|/Script/Engine.Character|GetCharacterMovement _asfirst_person_character))
  (CameraFades|StartCameraFade (Game|GetPlayerCameraManager 0) 0.0 1.0 5.0 "(R=0.000000,G=0.000000,B=0.000000,A=1.000000)" false true)
  (bind _drag (Timeline|PlayerDrag PlayFromStart)
    (:Update
      (Transformation|SetActorRelativeTransform _asfirst_person_character (Math|Transform|MakeTransform (Math|Vector|MakeVector (.x (Transformation|GetWorldLocation (Variables|/Script/Engine.Actor|GetRootComponent _asfirst_person_character))) (.y (Transformation|GetWorldLocation (Variables|/Script/Engine.Actor|GetRootComponent _asfirst_person_character))) _drag)) false false))
    (:Finished
      (Transformation|SetActorTransform _asfirst_person_character (Math|Transform|MakeTransform "-15782.000000,-5305.000000,-795.000000" "0, 0, 0" "1,1,1") false true)
      (CameraFades|StartCameraFade (Game|GetPlayerCameraManager 0) 1.0 0.0 5.0 "(R=0.000000,G=0.000000,B=0.000000,A=1.000000)" false true)
      (Pawn|Components|CharacterMovement|SetMovementMode (Variables|/Script/Engine.Character|GetCharacterMovement _asfirst_person_character) "MOVE_Swimming" 0))))

(event EventBeginPlay)

(event Collision|EventActorBeginOverlap
  (params (OtherActor :type Actor%20Object%20Reference))
  (Utilities|Casting|CastToFirstPersonCharacter OtherActor)
  (Variables|Default|SetStandingInPuddle true))

(event Collision|EventActorEndOverlap
  (params (OtherActor :type Actor%20Object%20Reference))
  (Utilities|Casting|CastToFirstPersonCharacter OtherActor)
  (Variables|Default|SetStandingInPuddle false))

(event EventTick
  (params (DeltaSeconds :type Float%20%28single-precision%29))
  (if (Variables|/Game/Blueprints/SinkEvent.SinkEvent_C|GetWaterIsLeaking (Variables|Default|GetSink))
    (Development|SetHiddeninGame (Variables|Default|GetWater_puddle) false false)))

(fn ConstructionScript)