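; Interactable door Blueprint that turns its knob and swings open or closed when OnInteract fires.
; Each interaction toggles the knob timeline between play and reverse, rolling the knob pivot.
; When that timeline finishes, the door timeline toggles direction to yaw the door pivot.
; Attached sounds play when the knob finishes at a nonzero angle and when the door finishes at zero yaw.
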(event EventBeginPlay)

(event Collision|EventActorBeginOverlap
  (params (OtherActor :type Actor%20Object%20Reference)))

(event EventTick
  (params (DeltaSeconds :type Float%20%28single-precision%29)))

(event EventOnInteract
  (bind _doorknobpivot (Variables|Default|GetDoorKnobPivot))
  (if (Variables|Default|GetDoorKnobOpen)
    (Variables|Default|SetDoorKnobOpen false)
    (bind _knobrot (Timeline|DoorKnobRot Play)
      (:Update
        (Transformation|SetRelativeRotation _doorknobpivot (Math|Rotator|MakeRotator _knobrot 0.0 0.0) false false))
      (:Finished
        (Utilities|FlowControl|Sequence
          (:then_0
            (if (Variables|Default|GetDoorOpen)
              (Variables|Default|SetDoorOpen false)
              (bind _doorrot (Timeline|DoorRotation Play)
                (:Update
                  (Transformation|SetRelativeRotation (Variables|Default|GetDoorPivot) (Math|Rotator|MakeRotator 0.0 0.0 _doorrot) false false))
                (:Finished
                  (if (== _doorrot 0.0)
                    (Audio|SpawnSoundAttached "/Game/Sounds/DoorCloses.DoorCloses" (Variables|Default|GetDoor) "None" "0, 0, 0" "0, 0, 0" "KeepRelativeOffset" false 3.0))))
              (else
                (Variables|Default|SetDoorOpen true)
                (Timeline|DoorRotation Reverse))))
          (:then_1
            (if (not (== _knobrot 0.0))
              (Audio|SpawnSoundAttached "/Game/Sounds/DoorKnob.DoorKnob" _doorknobpivot "None" "0, 0, 0" "0, 0, 0" "KeepRelativeOffset" false 5.0))))))
    (else
      (Variables|Default|SetDoorKnobOpen true)
      (Timeline|DoorKnobRot Reverse))))

(fn ConstructionScript)