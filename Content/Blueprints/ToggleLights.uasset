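; ToggleLights is an interactable that changes the lighting of the roof and wall lamps in its ActorLamps array.
; OnInteract plays the LightFlick timeline, whose LightIntensity track drives the point lights on each RoofLamp_BP and WallLamp.
; Each update also sets the lamps' dynamic material brightness parameters to zero.
; Despite the name, it only plays forward: the FlipFlop is unconnected, so nothing toggles back.
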(event EventBeginPlay)

(event Collision|EventActorBeginOverlap
  (params (OtherActor :type Actor%20Object%20Reference)))

(event EventTick
  (params (DeltaSeconds :type Float%20%28single-precision%29)))

(event EventOnInteract
  (bind _lightintensity (Timeline|LightFlick Play)
    (:Update
      (for _array_element (Variables|Default|GetActorLamps)
        (Utilities|FlowControl|Sequence
          (:then_0
            (bind _asroof_lamp_bp (Utilities|Casting|CastToRoofLamp_BP _array_element))
            (Rendering|Components|Light|SetIntensity (Variables|/Game/Blueprints/RoofLamp_BP.RoofLamp_BP_C|GetPointLight _asroof_lamp_bp) _lightintensity)
            (Rendering|Material|SetScalarParameterValue (Variables|/Game/Blueprints/RoofLamp_BP.RoofLamp_BP_C|GetRoofLamp_DynMat _asroof_lamp_bp) "RL_Brightness" 0.0 :!class /Script/Engine.MaterialInstanceDynamic))
          (:then_1
            (bind _aswall_lamp (Utilities|Casting|CastToWallLamp _array_element))
            (Rendering|Components|Light|SetIntensity (Variables|/Game/Blueprints/WallLamp.WallLamp_C|GetPointLight _aswall_lamp) _lightintensity)
            (Rendering|Material|SetScalarParameterValue (Variables|/Game/Blueprints/WallLamp.WallLamp_C|GetWallLamp_DynMat _aswall_lamp) "WL_Brightness" 0.0 :!class /Script/Engine.MaterialInstanceDynamic)))))))

(fn ConstructionScript)