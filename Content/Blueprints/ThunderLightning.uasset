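; Thunder and lightning actor that flashes a spotlight and plays thunder sounds once EnableLightning activates it.
; A delayed ThunderBolt timeline drives light intensity and leads into ThunderBoltRepeat, which replays after randomized delays.
; The repeat timeline's update chain alternates long and short sounds attached to the light, reseeding its random stream with a fixed seed each time.
; When Sink reports InWater, that chain only logs a message instead of scheduling another strike.
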(event Custom|EnableLightning
  (params (Activated :type Boolean))
  (bind _randomstream (Variables|Default|GetRandomStream))
  (bind _spotlight (Variables|Default|GetSpotLight))
  (bind _returnvalue (Math|Random|RandomFloatinRangefromStream 1e+01 15.0 _randomstream))
  (if Activated
    (Utilities|FlowControl|Delay 2.0)
    (bind _thunderintensity (Timeline|ThunderBolt Play)
      (:Update
        (Rendering|Components|Light|SetIntensity (Variables|Default|GetSpotLight) _thunderintensity)
        (Utilities|FlowControl|Delay 4.0)
        (Variables|Default|SetThunderAgain? true)
        (bind _thunderintensity_2 (Timeline|ThunderBoltRepeat PlayFromStart)
          (:Update
            (Rendering|Components|Light|SetIntensity (Variables|Default|GetSpotLight) _thunderintensity_2)
            (Utilities|FlowControl|Delay 2.0)
            (if (Variables|/Game/Blueprints/SinkEvent.SinkEvent_C|GetInWater? (Variables|Default|GetSink))
              (Development|PrintString "Yaaay!" false)
              (else
                (Variables|Default|SetThunderAgain? true)
                (Math|Random|SetRandomStreamSeed _randomstream 1)
                (switch int (Variables|Default|GetThunderSounds)
                  (:0
                    (Audio|SpawnSoundAttached "/Game/Sounds/ThunderLong.ThunderLong" _spotlight "None" "0, 0, 0" "0, 0, 0" "KeepRelativeOffset" false 0.2))
                  (:1
                    (Audio|SpawnSoundAttached "/Game/Sounds/ThunderShort.ThunderShort" _spotlight "None" "0, 0, 0" "0, 0, 0" "KeepRelativeOffset" false 0.2)))
                (bind _result (Math|Integer|IncrementInt (Variables|Default|GetThunderSounds))
                  (:%20%20
                    (if (> _result 1)
                      (Variables|Default|SetThunderSounds 0)
                      (Utilities|FlowControl|Delay _returnvalue)
                      (Timeline|ThunderBoltRepeat PlayFromStart)
                      (else
                        (Utilities|FlowControl|Delay _returnvalue)
                        (Timeline|ThunderBoltRepeat PlayFromStart)))))))))))))

(event EventBeginPlay)

(event Collision|EventActorBeginOverlap
  (params (OtherActor :type Actor%20Object%20Reference)))

(event EventTick
  (params (DeltaSeconds :type Float%20%28single-precision%29)))

(fn ConstructionScript)