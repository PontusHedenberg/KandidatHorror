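; Wall lamp Blueprint whose bulb can blow out once when its EventStarted event is called.
; The construction script creates a dynamic material instance on the lamp mesh for brightness control.
; EventStarted passes through a DoOnce, then stops the buzzing audio, plays the exploding bulb sound, and zeroes both the point light intensity and the material brightness parameter.
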(event Custom|EventStarted
  (Utilities|FlowControl|DoOnce false
    (:Completed
      (Audio|Components|Audio|Stop (Variables|Default|GetWallLightBuzzingAudio))
      (Audio|Components|Audio|Play (Variables|Default|GetExplodingLightbulb) 0.0)
      (Rendering|Components|Light|SetIntensity (Variables|Default|GetPointLight) 0.0)
      (Rendering|Material|SetScalarParameterValue (Variables|Default|GetWallLamp_DynMat) "WL_Brightness" 0.0 :!class /Script/Engine.MaterialInstanceDynamic))))

(event EventBeginPlay
  (|CallParentFunction) ; This node is disabled and will not be called.\nDrag off pins to build functionality.
)

(event Collision|EventActorBeginOverlap
  (params (OtherActor :type Actor%20Object%20Reference))
  (|CallParentFunction OtherActor) ; This node is disabled and will not be called.\nDrag off pins to build functionality.
)

(event EventTick
  (params (DeltaSeconds :type Float%20%28single-precision%29))
  (|CallParentFunction DeltaSeconds) ; This node is disabled and will not be called.\nDrag off pins to build functionality.
)

(fn ConstructionScript
  (|CallParentFunction)
  (bind _returnvalue (Rendering|Material|CreateDynamicMaterialInstance (Variables|Default|GetWall_lamp_Lamp) 0 0 :!class /Script/Engine.PrimitiveComponent))
  (Variables|Default|SetWallLamp_DynMat _returnvalue))