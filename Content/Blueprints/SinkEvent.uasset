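; Scripted sink event that starts a water leak after the lights go out and then lets the player trigger a teleporter.
; Tick polls EventManager.LightsOff, waits on a Delay, unhides the PSparks effect, then once attaches the leak sound and flags WaterIsLeaking.
; OnInteract requires the leak, darkness and Teleporter.StandingInPuddle, then once calls SinkActivated with the player character and sets InWater.
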(event EventBeginPlay)

(event Collision|EventActorBeginOverlap
  (params (OtherActor :type Actor%20Object%20Reference)))

(event EventTick
  (params (DeltaSeconds :type Float%20%28single-precision%29))
  (bind _p_sparks (Variables|Default|GetP_Sparks))
  (if (Variables|/Game/Blueprints/ToggleLights.ToggleLights_C|GetLightsOff (Variables|Default|GetEventManager))
    (Utilities|FlowControl|Delay 2e+01)
    (Development|SetHiddeninGame _p_sparks false false)
    (Utilities|FlowControl|DoOnce false
      (:Completed
        (Audio|SpawnSoundAttached "/Game/Sounds/WaterLeak.WaterLeak" _p_sparks "None" "0, 0, 0" "0, 0, 0" "KeepRelativeOffset" false 1.0 1.0 0.0 "/Game/NewSoundAttenuation.NewSoundAttenuation")
        (Variables|Default|SetWaterIsLeaking true)))))

(event EventOnInteract
  (bind _teleporter (Variables|Default|GetTeleporter))
  (if (and (Variables|Default|GetWaterIsLeaking) (Variables|/Game/Blueprints/ToggleLights.ToggleLights_C|GetLightsOff (Variables|Default|GetEventManager)))
    (if (Variables|/Game/Blueprints/PuddleTeleporter.PuddleTeleporter_C|GetStandingInPuddle _teleporter)
      (Utilities|FlowControl|DoOnce false
        (:Completed
          (Default|SinkActivated _teleporter (Game|GetPlayerCharacter 0))
          (Variables|Default|SetInWater? true))))))

(fn ConstructionScript)